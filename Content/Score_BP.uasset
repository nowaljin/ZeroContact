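; Score pickup actor that awards a point to the player when its static mesh registers a hit.
; The hit event adds one to the Score on BP_Player, spawns the NS_GridFigure Niagara effect at the mesh's transform, then destroys the actor.
; It does not check what caused the hit, so any collision credits player 0 and consumes the pickup.
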(event OnComponentHit(StaticMesh)
  (params (HitComponent :type Primitive%20Component%20Object%20Reference) (OtherActor :type Actor%20Object%20Reference) (OtherComp :type Primitive%20Component%20Object%20Reference) (NormalImpulse :type Vector :default "0, 0, 0") (Hit :type Hit%20Result%20Structure%20%28by%20ref%29))
  (bind _staticmesh (Variables|Default|GetStaticMesh))
  (Utilities|FlowControl|Sequence
    (:then_0
      (bind _asbp_player (Utilities|Casting|CastToBP_Player (Game|GetPlayerCharacter 0)))
      (Variables|/Game/Character/BP_Player.BP_Player_C|Setscore _asbp_player (+ (Variables|/Game/Character/BP_Player.BP_Player_C|Getscore _asbp_player) 1)))
    (:then_1
      (Niagara|SpawnSystematLocation "/Game/FreeNiagaraPack/Effects/NS_GridFigure.NS_GridFigure" (Transformation|GetWorldLocation _staticmesh) (Transformation|GetWorldRotation _staticmesh) (Variables|Default|GetScale)))
    (:then_2
      (Actor|DestroyActor))))

(event EventBeginPlay)

(event Collision|EventActorBeginOverlap
  (params (OtherActor :type Actor%20Object%20Reference)))

(event EventTick
  (params (DeltaSeconds :type Float%20%28single-precision%29)))

(fn ConstructionScript)